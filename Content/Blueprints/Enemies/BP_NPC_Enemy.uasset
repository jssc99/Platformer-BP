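; Enemy NPC that roams, chases the player, deals contact damage and can drop a life heart on death.
; MoveNPC loops random navigable moves within a radius, while PawnSensing sends it after a sighted BP_Player via AIMoveTo.
; DamageCube overlaps subtract player life, and LifeCube overlaps launch the player away from the cube.
; AIDeath, not called here, decrements enemy life and, on its threshold check, spawns BP_LifeHeart and destroys the actor.
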(event `self.ReceiveBeginPlay`
  (`self.MoveNPC`))

(event `MoveNPC`
  (bind _output_get (set `self.Random Location` (`NavigationSystemV1.K2_GetRandomReachablePointInRadius` (`self.K2_GetActorLocation`) 1500.0 null null)))
  (`|AIMoveTo` self _output_get null
    (:`OnSuccess`
      (`KismetSystemLibrary.Delay` 2.0)
      (`self.MoveNPC`))
    (:`OnFail`
      (`KismetSystemLibrary.Delay` 0.2)
      (`self.MoveNPC`)))
  (if (stale _output_get_2)
    (bind _asbp_player (cast `/Game/Blueprints/Player/BP_Player` (stale `self.PawnSensing.OnSeePawn` Pawn) :!label _label))
    (bind _output_get_2 (set `self.FoundPlayer` true))
    (`|AIMoveTo` self (0.0 0.0 0.0) _asbp_player 10.0)
    (else
      (set `self.FoundPlayer` false))))

(event `self.PawnSensing.OnSeePawn`
  (params (Pawn :type "Pawn Object Reference"))
  (goto _label))

(event `self.DamageCube.OnComponentBeginOverlap`
  (params (OverlappedComponent :type "PrimitiveComponent Object Reference") (OtherActor :type "Actor Object Reference") (OtherComp :type "PrimitiveComponent Object Reference") (OtherBodyIndex :type Integer) (bFromSweep :type Boolean) (SweepResult :type "HitResult Structure (by ref)"))
  ;[1 1 1] DamageToPlayer
  (bind _asbp_player (cast `/Game/Blueprints/Player/BP_Player` OtherActor))
  (set `/Game/Blueprints/Player/BP_Player.PlayerLife` (- (`/Game/Blueprints/Player/BP_Player.PlayerLife` _asbp_player) 1) _asbp_player))

(event `self.LifeCube.OnComponentBeginOverlap`
  (params (OverlappedComponent :type "PrimitiveComponent Object Reference") (OtherActor :type "Actor Object Reference") (OtherComp :type "PrimitiveComponent Object Reference") (OtherBodyIndex :type Integer) (bFromSweep :type Boolean) (SweepResult :type "HitResult Structure (by ref)"))
  ;[1 1 1] Directional Bumper
  (bind _asbp_player (cast `/Game/Blueprints/Player/BP_Player` OtherActor))
  (`self.LaunchCharacter` _asbp_player (* (`KismetMathLibrary.Normal` (- (`self.K2_GetActorLocation` _asbp_player) (`SceneComponent.K2_GetComponentLocation` (`self.LifeCube`))) 0.1) (`self.LaunchVelocity`)) true true))

(fn `AIDeath`
  (bind _returnvalue (- (`self.AIEnemyLife`) 1))
  (set `self.AIEnemyLife` _returnvalue)
  (if (== _returnvalue 0)
    (`|SpawnActorFromClass` "/Game/Blueprints/UI/BP_LifeHeart.BP_LifeHeart_C" (`self.GetTransform`) "Undefined" "MultiplyWithRoot" null null)
    (`self.K2_DestroyActor`)
    (else
      (return))))

(fn `UserConstructionScript`)