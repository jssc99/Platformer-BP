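; BP_FEnemy is an AI enemy that hunts the player and drops a BP_LifeHeart on death.
; AI perception writes the sensed actor to the PlayerActor blackboard key and clears it on a timer after sight or sensing is lost.
; Box overlap costs the player a life, while LifeCube overlap launches them away.
; PlayerAttack spawns angled projectiles at random points overhead; PlayerDash adds only zero movement input.
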(event `self.AIPerception.OnTargetPerceptionUpdated`
  (params (Actor :type "Actor Object Reference") (Stimulus :type "AIStimulus Structure"))
  (if Stimulus_bSuccessfullySensed
    (`self.AISetPlayerActor` Actor)
    (`KismetSystemLibrary.PrintString` "Found player")
    (else
      (bind _returnvalue (`KismetSystemLibrary.K2_SetTimer` null "AIForgetPlayerActor" 4.0))
      (set `self.ForgetTimer` _returnvalue)
      (`KismetSystemLibrary.PrintString` "Patrolling"))))

(event `self.Box.OnComponentBeginOverlap`
  (params (OverlappedComponent :type "PrimitiveComponent Object Reference") (OtherActor :type "Actor Object Reference") (OtherComp :type "PrimitiveComponent Object Reference") (OtherBodyIndex :type Integer) (bFromSweep :type Boolean) (SweepResult :type "HitResult Structure (by ref)"))
  ;[1 1 1] DamageToPlayer
  (bind _asbp_player (cast `/Game/Blueprints/Player/BP_Player` OtherActor))
  (bind _output_get (set `/Game/Blueprints/Player/BP_Player.PlayerLife` (- (`/Game/Blueprints/Player/BP_Player.PlayerLife` _asbp_player) 1) _asbp_player))
  (`KismetSystemLibrary.PrintString` (`KismetStringLibrary.Conv_IntToString` _output_get)))

(event `self.LifeCube.OnComponentBeginOverlap`
  (params (OverlappedComponent :type "PrimitiveComponent Object Reference") (OtherActor :type "Actor Object Reference") (OtherComp :type "PrimitiveComponent Object Reference") (OtherBodyIndex :type Integer) (bFromSweep :type Boolean) (SweepResult :type "HitResult Structure (by ref)"))
  ;[1 1 1] Directional Bumper
  (bind _asbp_player (cast `/Game/Blueprints/Player/BP_Player` OtherActor))
  (`self.LaunchCharacter` _asbp_player (* (`KismetMathLibrary.Normal` (- (`self.K2_GetActorLocation` _asbp_player) (`SceneComponent.K2_GetComponentLocation` (`self.LifeCube`))) 0.1) (`self.LaunchVelocity`)) true true))

(fn `AIDeath`
  (bind _returnvalue (- (`self.AIEnemyLife`) 1))
  (set `self.AIEnemyLife` _returnvalue)
  (if (== _returnvalue 0)
    (`|SpawnActorFromClass` "/Game/Blueprints/UI/BP_LifeHeart.BP_LifeHeart_C" (`self.GetTransform`) "Undefined" "MultiplyWithRoot" null null)
    (`self.K2_DestroyActor`)
    (else
      (return))))

(fn `AIForgetPlayerActor`
  (`self.AISetPlayerActor` null)
  (return))

(fn `AISetPlayerActor`
  (params (actor :type "Actor Object Reference"))
  (`KismetSystemLibrary.K2_ClearAndInvalidateTimerHandle` (`self.ForgetTimer`))
  (`BlackboardComponent.SetValueAsObject` (`AIBlueprintHelperLibrary.GetBlackboard` null) "PlayerActor" actor)
  (return))

(fn `PlayerAttack`
  (bind (_returnvalue_x _returnvalue_y _returnvalue_z) (`KismetMathLibrary.BreakVector` (`self.K2_GetActorLocation`)))
  (bind (_returnvalue_roll _returnvalue_pitch _returnvalue_yaw) (`KismetMathLibrary.BreakRotator` (`self.K2_GetActorRotation`)))
  ;[1 1 1] PlayerAttack
  (`|SpawnActorFromClass` "/Game/Blueprints/Player/BP_Projectle.BP_Projectle_C" (`KismetMathLibrary.MakeTransform` (`KismetMathLibrary.MakeVector` (`KismetMathLibrary.Conv_IntToDouble` (`KismetMathLibrary.RandomIntegerInRange` (`KismetMathLibrary.FTrunc` (- _returnvalue_x 300.0)) (`KismetMathLibrary.FTrunc` (+ _returnvalue_x 300.0)))) (`KismetMathLibrary.Conv_IntToDouble` (`KismetMathLibrary.RandomIntegerInRange` (`KismetMathLibrary.FTrunc` (- _returnvalue_y 300.0)) (`KismetMathLibrary.FTrunc` (+ _returnvalue_y 300.0)))) (+ _returnvalue_z 700.0)) (`KismetMathLibrary.MakeRotator` 0.0 -45.0 _returnvalue_yaw)) "AlwaysSpawn" "MultiplyWithRoot" null null))

(fn `PlayerDash`
  (`self.AddMovementInput` (0.0 0.0 0.0)))

(fn `UserConstructionScript`)