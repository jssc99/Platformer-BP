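; BP_Enemy is an enemy Blueprint that reacts to AI perception by updating a PlayerActor blackboard key.
; A successful sense calls AISetPlayerActor, which cancels the forget timer and writes the key, though no actor argument is supplied in that call.
; A lost sense starts a short delay before AIForgetPlayerActor calls the same setter with an empty actor to clear the key.
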(event `self.AIPerception.OnTargetPerceptionUpdated`
  (params (Actor :type "Actor Object Reference") (Stimulus :type "AIStimulus Structure"))
  (if Stimulus_bSuccessfullySensed
    (`self.AISetPlayerActor` null)
    (`KismetSystemLibrary.PrintString` "Found player")
    (else
      (bind _returnvalue (`KismetSystemLibrary.K2_SetTimer` null "AIForgetPlayerActor" 4.0))
      (set `self.ForgetTimer` _returnvalue)
      (`KismetSystemLibrary.PrintString` "Patrolling"))))

(fn `AIForgetPlayerActor`
  (`self.AISetPlayerActor` null)
  (return))

(fn `AISetPlayerActor`
  (params (actor :type "Actor Object Reference"))
  (`KismetSystemLibrary.K2_ClearAndInvalidateTimerHandle` (`self.ForgetTimer`))
  (`BlackboardComponent.SetValueAsObject` (`AIBlueprintHelperLibrary.GetBlackboard` null) "PlayerActor" actor)
  (return))

(fn `UserConstructionScript`)