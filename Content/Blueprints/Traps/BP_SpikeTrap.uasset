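; BP_SpikeTrap is a trap actor that drains the player's life while they stand on its Hitbox.
; Hitbox begin-overlap and a Tick check for overlapping BP_Player actors share one damage chain.
; That chain casts the begin-overlap event's OtherActor to BP_Player, waits on a half-second Delay, then decrements PlayerLife.
; Tick re-enters the Delay each frame, so damage repeats periodically during overlap.
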(event `self.ReceiveTick`
  (params (DeltaSeconds :type "Float (single-precision)"))
  ;[1 1 1] Main Loop
  ;;[1 1 1] IF player is on trap
  (if (`KismetMathLibrary.Conv_IntToBool` (`KismetArrayLibrary.Array_Length` (`PrimitiveComponent.GetOverlappingActors` (`self.Hitbox`) "/Game/Blueprints/Player/BP_Player.BP_Player_C")))
    ;;[1 1 1] Damage Player
    (bind _asbp_player (cast `/Game/Blueprints/Player/BP_Player` (stale `self.Hitbox.OnComponentBeginOverlap` OtherActor) :!label _label))
    (`KismetSystemLibrary.Delay` 0.5)
    (set `/Game/Blueprints/Player/BP_Player.PlayerLife` (- (`/Game/Blueprints/Player/BP_Player.PlayerLife` _asbp_player) 1) _asbp_player)))

(event `self.Hitbox.OnComponentBeginOverlap`
  (params (OverlappedComponent :type "PrimitiveComponent Object Reference") (OtherActor :type "Actor Object Reference") (OtherComp :type "PrimitiveComponent Object Reference") (OtherBodyIndex :type Integer) (bFromSweep :type Boolean) (SweepResult :type "HitResult Structure (by ref)"))
  ;[1 1 1] Main Loop
  ;;[1 1 1] Damage Player
  (goto _label))

(fn `UserConstructionScript`)