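; Falling platform trap that drops after something overlaps its hitbox, then respawns.
; On overlap, after a short delay, it stores the platform's relative transform, nudges it down and starts a timer in Tick.
; Tick enables physics simulation once the fall threshold passes.
; At the respawn threshold it stops physics, teleports the platform to the stored values as world location and rotation, and rearms.
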(event `self.Hitbox.OnComponentBeginOverlap`
  (params (OverlappedComponent :type "PrimitiveComponent Object Reference") (OtherActor :type "Actor Object Reference") (OtherComp :type "PrimitiveComponent Object Reference") (OtherBodyIndex :type Integer) (bFromSweep :type Boolean) (SweepResult :type "HitResult Structure (by ref)"))
  (bind (_returnvalue_location _returnvalue_rotation) (`KismetMathLibrary.BreakTransform` (`SceneComponent.GetRelativeTransform` (`self.Platform`))))
  ;[1 1 1] Player Collision Detection
  (if (!= (`self.isFalling`) true)
    (`KismetSystemLibrary.Delay` 0.5)
    (set `self.isFalling` true)
    (set `self.BaseLoc` _returnvalue_location)
    (set `self.BaseRot` _returnvalue_rotation)
    (`SceneComponent.K2_AddRelativeLocation` (`self.Platform`) (0.0 0.0 -10.0) false false)))

(event `self.ReceiveTick`
  (params (DeltaSeconds :type "Float (single-precision)"))
  (bind _platform (`self.Platform`))
  ;[1 1 1] Main Loop
  ;;[1 1 1] IF falling: Increase timer
  (if (`self.isFalling`)
    ;;[1 1 1] IF platform has to be reset
    (bind _output_get (set `self.Timer` (+ (`self.Timer`) DeltaSeconds)))
    (if (>= _output_get (`self.TimeBeforeRespawn`))
      ;;[1 1 1] Reset Pos, Rot, Timer, isFalling, and stop physics
      (`SceneComponent.K2_SetWorldLocationAndRotation` _platform (`self.BaseLoc`) (`self.BaseRot`) false true)
      (`PrimitiveComponent.SetSimulatePhysics` _platform false)
      (set `self.Timer` 0.0)
      (set `self.isFalling` false)
      (else
        ;;[1 1 1] IF platform has to start falling
        (if (and (>= (`self.Timer`) (`self.TimeBeforeFall`)) (!= (`SceneComponent.IsSimulatingPhysics` (`self.Platform`) "None") true))
          ;;[1 1 1] Start physics
          (`PrimitiveComponent.SetSimulatePhysics` (`self.Platform`) true))))))

(fn `UserConstructionScript`)