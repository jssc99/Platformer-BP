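; BP_FireTrap is a looping trap that warns with smoke, then shoots fire and takes life from BP_Player.
; Tick advances a timer that switches the smoke and fire particles at start/end thresholds and resets when fire ends.
; During fire, a Hitbox overlap check feeds a half-second Delay that subtracts one PlayerLife.
; Hitbox begin overlap enters the same damage path regardless of phase, and its OtherActor is the damage target.
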(event `self.ReceiveTick`
  (params (DeltaSeconds :type "Float (single-precision)"))
  (bind _timer (`self.Timer`))
  ;[1 1 1] Main Loop
  ;;[1 1 1] Increment timer
  ;;[1 1 1] IF fire has to end
  (bind _output_get (set `self.Timer` (+ DeltaSeconds (`self.Timer`))))
  (if (>= _output_get (`self.FireEnd`))
    ;;[1 1 1] Stop fire, reset timer
    (`ActorComponent.Deactivate` (`self.P_Fire`))
    (set `self.Timer` 0.0)
    (else
      ;;[1 1 1] IF fire can start and fire has not already started
      (if (and (>= (`self.Timer`) (`self.FireStart`)) (!= (`ActorComponent.IsActive` (`self.P_Fire`)) true))
        ;;[1 1 1] Activate fire, stop smoke
        (`ActorComponent.Activate` (`self.P_Fire`) false)
        (`ActorComponent.Deactivate` (`self.P_Smoke`))
        (else
          ;;[1 1 1] IF fire has started and has not ended
          (if (and (>= (`self.FireEnd`) _timer) (>= _timer (`self.FireStart`)))
            ;;[1 1 1] IF player is on trap
            (if (`KismetMathLibrary.Conv_IntToBool` (`KismetArrayLibrary.Array_Length` (`PrimitiveComponent.GetOverlappingActors` (`self.Hitbox`) "/Game/Blueprints/Player/BP_Player.BP_Player_C")))
              ;;[1 1 1] Damage Player
              (bind _asbp_player (cast `/Game/Blueprints/Player/BP_Player` (stale `self.Hitbox.OnComponentBeginOverlap` OtherActor) :!label _label))
              (`KismetSystemLibrary.Delay` 0.5)
              (set `/Game/Blueprints/Player/BP_Player.PlayerLife` (- (`/Game/Blueprints/Player/BP_Player.PlayerLife` _asbp_player) 1) _asbp_player))
            (else
              ;;[1 1 1] IF smoke can start and has not already started
              (if (and (>= (`self.Timer`) (`self.SmokeStart`)) (!= (`ActorComponent.IsActive` (`self.P_Smoke`)) true))
                ;;[1 1 1] Activate smoke
                (`ActorComponent.Activate` (`self.P_Smoke`) false)))))))))

(event `self.Hitbox.OnComponentBeginOverlap`
  (params (OverlappedComponent :type "PrimitiveComponent Object Reference") (OtherActor :type "Actor Object Reference") (OtherComp :type "PrimitiveComponent Object Reference") (OtherBodyIndex :type Integer) (bFromSweep :type Boolean) (SweepResult :type "HitResult Structure (by ref)"))
  ;[1 1 1] Main Loop
  ;;[1 1 1] Damage Player
  (goto _label))

(fn `UserConstructionScript`)