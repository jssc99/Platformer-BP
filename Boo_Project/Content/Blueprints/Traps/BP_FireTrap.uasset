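; BP_FireTrap is a timed trap that loops through idle, smoke warning and fire particle effects.
; Tick accumulates a timer against SmokeStart, FireStart and FireEnd, though the smoke check can reactivate smoke while fire burns.
; A box overlap by BP_Player during active fire only prints a debug message, with no damage applied.
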(event `self.Box.OnComponentBeginOverlap`
  (params (OverlappedComponent :type "PrimitiveComponent Object Reference") (OtherActor :type "Actor Object Reference") (OtherComp :type "PrimitiveComponent Object Reference") (OtherBodyIndex :type Integer) (bFromSweep :type Boolean) (SweepResult :type "HitResult Structure (by ref)"))
  ;[1 1 1] Basic Fire Trap
  (cast `/Game/Blueprints/BP_Player` OtherActor)
  (if (`ActorComponent.IsActive` (`self.P_Fire`))
    (`KismetSystemLibrary.PrintText` "Fire trap activated")))

(event `self.ReceiveTick`
  (params (DeltaSeconds :type "Float (single-precision)"))
  ;[1 1 1] Nothing to Smoke to Fire to Nothing: The Loop
  (bind _output_get (set `self.Timer` (+ DeltaSeconds (`self.Timer`))))
  ;;[1 1 1] End fire, reset timer
  (if (>= _output_get (`self.FireEnd`))
    (`ActorComponent.Deactivate` (`self.P_Fire`))
    (set `self.Timer` 0.0)
    (else
      ;;[1 1 1] Activate fire, end smoke
      (if (and (>= (`self.Timer`) (`self.FireStart`)) (!= (`ActorComponent.IsActive` (`self.P_Fire`)) true))
        (`ActorComponent.Activate` (`self.P_Fire`) false)
        (`ActorComponent.Deactivate` (`self.P_Smoke`))
        (else
          ;;[1 1 1] Activate smoke
          (if (and (>= (`self.Timer`) (`self.SmokeStart`)) (!= (`ActorComponent.IsActive` (`self.P_Smoke`)) true))
            (`ActorComponent.Activate` (`self.P_Smoke`) false)))))))

(fn `UserConstructionScript`)